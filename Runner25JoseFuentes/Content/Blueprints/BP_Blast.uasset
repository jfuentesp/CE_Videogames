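; BP_Blast is a moving obstacle that scrolls along negative X, scores points for the player and kills on impact.
; Tick teleport-free, sweepless location updates move it at MSpeed, scaled by delta time.
; Any Trigger overlap passes MScoreValueToAdd to BP_GameMode's score call, with no actor filter or destroy step.
; A Box hit calls the game mode's player death, guarded by DoOnce so it fires only once.
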(event `self.ReceiveTick`
  (params (DeltaSeconds :type "Float (single-precision)"))
  ;[0.2088 0.8801 1] Movement
  (`self.K2_SetActorLocation` (+ (`self.K2_GetActorLocation`) (* DeltaSeconds (* (-1.0 0.0 0.0) (`self.mSpeed`))))))

(event `self.Trigger.OnComponentBeginOverlap`
  (params (OverlappedComponent :type "PrimitiveComponent Object Reference") (OtherActor :type "Actor Object Reference") (OtherComp :type "PrimitiveComponent Object Reference") (OtherBodyIndex :type Integer) (bFromSweep :type Boolean) (SweepResult :type "HitResult Structure (by ref)"))
  ;[0.969 1 0.3804] Score Increase and Destroy
  (bind _asbp_game_mode (cast `/Game/Blueprints/BP_GameMode` (`GameplayStatics.GetGameMode`)))
  (`/Game/Blueprints/BP_GameMode.OnPlayerScoreRaises` _asbp_game_mode (`self.mScoreValueToAdd`)))

(event `self.Box.OnComponentHit`
  (params (HitComponent :type "PrimitiveComponent Object Reference") (OtherActor :type "Actor Object Reference") (OtherComp :type "PrimitiveComponent Object Reference") (NormalImpulse :type "Vector Structure") (Hit :type "HitResult Structure (by ref)"))
  ;[1 0.05782 0.1475] Collision with Player (Death trigger)
  (`/Engine/EditorBlueprintResources/StandardMacros.DoOnce` false
    (:`Completed`
      (bind _asbp_game_mode (cast `/Game/Blueprints/BP_GameMode` (`GameplayStatics.GetGameMode`)))
      (`/Game/Blueprints/BP_GameMode.OnPlayerDeath` _asbp_game_mode))))

(fn `UserConstructionScript`)