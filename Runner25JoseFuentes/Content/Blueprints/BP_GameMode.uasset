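; Game mode Blueprint that handles player death and keeps the running score.
; On BeginPlay it binds handlers to the player death and score-raise event dispatchers.
; Death calls the game-over dispatcher after a short delay, while each score event adds its points to the stored score and prints the new total as debug text.
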(event `self.ReceiveBeginPlay`
  (`|ExecutionSequence`
    (:`then_0`
      ;[0.5521 0.3077 0.3077] Player Death Event
      (add `self.OnPlayerDeath` (delegate `OnPlayerDeath_Event`)))
    (:`then_1`
      ;[1 0.9617 0.4222] Player Score Handler
      (add `self.OnPlayerScoreRaises` (delegate `OnPlayerScoreRaises_Event`)))))

(event `OnPlayerDeath_Event`
  ;[0.5521 0.3077 0.3077] Player Death Event
  (`KismetSystemLibrary.Delay` 2.0)
  (`self.OnGameOver`))

(event `OnPlayerScoreRaises_Event` :!signature `self.OnPlayerScoreRaises`
  (params (aPoints :type Integer))
  ;[1 0.9617 0.4222] Player Score Handler
  (bind _output_get (set `self.mScore` (+ aPoints (`self.mScore`))))
  (`KismetSystemLibrary.PrintString` (`KismetStringLibrary.Conv_IntToString` _output_get)))

(fn `UserConstructionScript`)