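; BP_Player is the Paper2D player character, with jump input and state-driven flipbook animation.
; BeginPlay adds the IMC_Base Enhanced Input context after a short delay and binds to BP_GameMode's player death dispatcher.
; While alive, Tick picks the run, jump or fall flipbook from ground state and vertical velocity.
; On death it stops those updates, shows the damage flipbook and disables input; despite the Death comment, nothing destroys the actor.
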(event `self.ReceiveBeginPlay`
  ;[1 1 1] Controller Handler
  (`|ExecutionSequence`
    (:`then_0`
      (`KismetSystemLibrary.Delay` 1.0)
      (bind _asplayer_controller (cast `PlayerController` (`self.GetController`)))
      (message `EnhancedInputSubsystemInterface.AddMappingContext` (pcsubsystem `EnhancedInputLocalPlayerSubsystem` _asplayer_controller) "/Game/Inputs/IMC_Base.IMC_Base" 0 (struct)))
    (:`then_1`
      ;[1 0.3097 0.3694] Death Handler
      (bind _asbp_game_mode (cast `/Game/Blueprints/BP_GameMode` (`GameplayStatics.GetGameMode`)))
      (add `/Game/Blueprints/BP_GameMode.OnPlayerDeath` _asbp_game_mode (delegate `OnPlayerDeath_Event`)))))

(event `OnPlayerDeath_Event`
  ;[1 0.3097 0.3694] Death Handler
  (set `self.mIsAlive` false)
  (`self.Death`))

(event `self.ReceiveTick`
  (params (DeltaSeconds :type "Float (single-precision)"))
  ;[1 1 1] Animation handler
  (if (`self.mIsAlive`)
    (`self.UpdateAnimation`)))

(event `EnhancedInput|/Game/Inputs/IA_Jump`
  (params (ActionValue :type Boolean) (ElapsedSeconds :type "Float (double-precision)") (TriggeredSeconds :type "Float (double-precision)") (InputAction :type "InputAction Object Reference" :default "/Game/Inputs/IA_Jump.IA_Jump"))
  ;[0.5089 0.3712 0.5149] Jump Action
  (:`Started`
    (`self.Jump`))
  (:`Completed`
    (`self.StopJumping`)))

(fn `Death`
  ;[1 0.2289 0.8918] Disables the player input, shows dead animation and destroys the actor after a delay
  (`|ExecutionSequence`
    (:`then_0`
      (`PaperFlipbookComponent.SetFlipbook` (`self.Sprite`) "/Game/Tileset/Sprites/Player/TakeDamage/PF_TakeDamage.PF_TakeDamage"))
    (:`then_1`
      (`self.DisableInput` (`GameplayStatics.GetPlayerController` 0)))))

(fn `UpdateAnimation`
  ;[0.6775 0.4947 1] If player is on ground...
  (if (`NavMovementComponent.IsMovingOnGround` (`self.CharacterMovement`))
    ;[1 0.6162 0.2634] Running animation is set as Player sprite.
    (`PaperFlipbookComponent.SetFlipbook` (`self.Sprite`) "/Game/Tileset/Sprites/Player/Move/PF_Run.PF_Run")
    (elif (> (.z (`self.GetVelocity`)) 0.0)
      ;[1 0.7206 0.3061] Jump animation is set as Player sprite.
      (`PaperFlipbookComponent.SetFlipbook` (`self.Sprite`) "/Game/Tileset/Sprites/Player/Jump/PF_Jump.PF_Jump")
      (else
        ;[1 0.7565 0.4511] Fall animation is set as Player sprite.
        (`PaperFlipbookComponent.SetFlipbook` (`self.Sprite`) "/Game/Tileset/Sprites/Player/Fall/PF_Fall.PF_Fall")))))

(fn `UserConstructionScript`)